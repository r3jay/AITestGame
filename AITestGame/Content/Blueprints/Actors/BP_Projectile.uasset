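; BP_Projectile is a projectile actor that damages whatever it overlaps and then destroys itself.
; On BeginPlay it starts a one-shot TimeToLive timer and caches its owner as the instigating controller, printing a message if the owner is not one.
; The construction script scales the collision sphere by Size and binds its begin-overlap event.
; The overlap handler applies Damage credited to that controller, without filtering the other actor.
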(event Custom|HandleOverlap
  (params (OverlappedComponent :type Primitive%20Component%20Object%20Reference) (OtherActor :type Actor%20Object%20Reference) (OtherComp :type Primitive%20Component%20Object%20Reference) (OtherBodyIndex :type Integer) (bFromSweep :type Boolean) (SweepResult :type Hit%20Result%20Structure%20%28by%20ref%29))
  ;[1 1 1] Week2
  (Game|Damage|ApplyDamage OtherActor (Variables|Default|GetDamage) (Variables|Default|GetOwnerController) self)
  (Actor|DestroyActor))

(event EventBeginPlay
  ;[1 1 1] Week2
  (Utilities|Time|SetTimerbyEvent (EventDispatchers|CreateEvent :!event K2DestroyActor) (Variables|Default|GetTimeToLive))
  (bind _ascontroller (Utilities|Casting|CastToController (Components|GetOwner))
    (:then
      (Variables|Default|SetOwnerController _ascontroller))
    (:CastFailed
      (Development|PrintString "Our owner is not a controller"))))

(fn ConstructionScript
  (Collision|BindEventtoOnComponentBeginOverlap (Variables|Default|GetSphereCollision) (EventDispatchers|CreateEvent :!event Custom|HandleOverlap))
  (Transformation|SetWorldScale3D (Variables|Default|GetSphereCollision) (Variables|Default|GetSize)))