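; AI-controlled agent character that bridges its weapon and health component to its AI controller.
; On BeginPlay it tints the mesh, binds weapon, hurt and death-animation delegates, and reloads ammo.
; Update events write health ratio and current ammo to the Blackboard, while EndAttack sends an AI message to itself.
; AgentAttack and AgentReload events forward attack and reload requests to the weapon.
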(event Custom|EndAttack
  ;[1 1 1] Week 1
  (Class|AIBlueprintHelperLibrary|SendAIMessage self (Variables|Default|GetAIMessage) 0 true))

(event Custom|UpdateBlackboardHealth
  (params (Ratio :type Float%20%28single-precision%29))
  ;[1 1 1] Week 1
  (AI|Components|Blackboard|SetValueasFloat (Variables|/Script/AIModule.AIController|GetBlackboard (AI|GetAIController self)) (Variables|Default|GetHealthRatioKey) Ratio))

(event Custom|UpdateBlackboardAmmo
  (params (Current :type Float%20%28single-precision%29) (Max :type Float%20%28single-precision%29))
  ;[1 1 1] Week 2
  (AI|Components|Blackboard|SetValueasFloat (Variables|/Script/AIModule.AIController|GetBlackboard (AI|GetAIController self)) (Variables|Default|GetAmmoKey) Current))

(event EventBeginPlay
  (bind _weapon (Variables|Default|GetWeapon))
  (|CallParentFunction)
  (Rendering|Material|SetVectorParameterValueonMaterials (Variables|Character|GetMesh) (Variables|Default|GetParameterName) (Math|Conversions|ToVector(LinearColor) (Variables|Default|GetColor)))
  ;[1 1 1] Week 1
  (EventDispatchers|BindEventtoOnActionStopped (Variables|Default|GetWeapon) (EventDispatchers|CreateEvent :!event Custom|EndAttack))
  (EventDispatchers|BindEventtoOnHurt (Variables|Default|GetHealthComponent) (EventDispatchers|CreateEvent :!event Custom|UpdateBlackboardHealth))
  (CallFunction|UpdateBlackboardHealth 1.0)
  ;[1 1 1] Week2
  (EventDispatchers|BindEventtoOnAmmoChange _weapon (EventDispatchers|CreateEvent :!event Custom|UpdateBlackboardAmmo))
  (Default|ReloadAmmo _weapon)
  (EventDispatchers|BindEventtoOnDeathEnded (Variables|Default|GetAs%20ABP%20Character%20Animation) (EventDispatchers|CreateEvent :!event K2DestroyActor)))

(event Collision|EventActorBeginOverlap
  (params (OtherActor :type Actor%20Object%20Reference)))

(event EventAgentReload
  ;[1 1 1] Week 2
  (Default|RequestReload (Variables|Default|GetWeapon)))

(event EventAgentAttack
  ;[1 1 1] Week 1
  (Default|Attack (Variables|Default|GetWeapon)))

(fn ConstructionScript
  (|CallParentFunction))