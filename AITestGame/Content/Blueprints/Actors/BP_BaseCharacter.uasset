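; Base character Blueprint that equips a rifle through a child actor and connects it to the character's animation and health.
; On BeginPlay it spawns the weapon class, caches the rifle and anim instance, destroying itself if either cast fails.
; It binds weapon fire and reload, hurt, death and animation reload events.
; Death plays an animation, disables collision and notifies the weapon; CanPickupHealth returns false by default.
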(event Custom|HandleDeath
  (params (Percent :type Float%20%28single-precision%29))
  (Default|DeadAnimation (Variables|Default|GetAs%20ABP%20Character%20Animation) 0.0)
  (Collision|SetActorEnableCollision false)
  (Default|OwnerDied (Variables|Default|GetWeapon)))

(event EventBeginPlay
  (bind _childactor (Variables|Default|GetChildActor))
  (bind _healthcomponent (Variables|Default|GetHealthComponent))
  (ChildActorComponent|SetChildActorClass _childactor (Variables|Default|GetWeaponClass))
  (bind _asbp_rifle (Utilities|Casting|CastToBP_Rifle (Variables|/Script/Engine.ChildActorComponent|GetChildActor _childactor))
    (:then
      (Variables|Default|SetWeapon _asbp_rifle)
      (bind _asabp_character_animation (Utilities|Casting|CastToABP_CharacterAnimation (Components|SkeletalMesh|GetAnimInstance (Variables|Character|GetMesh)))
        (:then
          (Variables|Default|SetAs%20ABP%20Character%20Animation _asabp_character_animation)
          (EventDispatchers|BindEventtoOnWeaponFired (Variables|Default|GetWeapon) (EventDispatchers|CreateEvent (Variables|Default|GetAs%20ABP%20Character%20Animation) :!event AttackAnimation))
          (EventDispatchers|BindEventtoOnHurt _healthcomponent (EventDispatchers|CreateEvent (Variables|Default|GetAs%20ABP%20Character%20Animation) :!event HurtAnimation))
          ;[1 1 1] Week 2
          (EventDispatchers|BindEventtoOnDead _healthcomponent (EventDispatchers|CreateEvent :!event Custom|HandleDeath))
          (EventDispatchers|BindEventtoOnReloadStart (Variables|Default|GetWeapon) (EventDispatchers|CreateEvent (Variables|Default|GetAs%20ABP%20Character%20Animation) :!event ReloadAnimation))
          (EventDispatchers|BindEventtoOnReloadEnd (Variables|Default|GetAs%20ABP%20Character%20Animation) (EventDispatchers|CreateEvent (Variables|Default|GetWeapon) :!event ActionStopped))
          (EventDispatchers|BindEventtoOnReloadNow (Variables|Default|GetAs%20ABP%20Character%20Animation) (EventDispatchers|CreateEvent (Variables|Default|GetWeapon) :!event ReloadAmmo)))
        (:CastFailed
          (Development|PrintString "We need an animation for the character")
          (Actor|DestroyActor))))
    (:CastFailed
      (Development|PrintString "We need a weapon for the character")
      (Actor|DestroyActor))))

(fn ConstructionScript)

(fn CanPickupHealth
  (params (OtherActor :type Actor%20Object%20Reference))
  (return false))