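; Player character Blueprint, built on a parent character class, that handles input for movement, camera look, attacking and reloading.
; On BeginPlay it creates the HUD, binds health, weapon ammo and death-animation events, and reloads the weapon, destroying itself without a player controller.
; Movement follows control yaw, and attack and reload delegate to the Weapon.
; Death and winning remove the HUD and disable input; health pickup is always allowed.
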(event Custom|WinGame
  (Widget|RemovefromParent (Variables|Default|GetHUDObject))
  (Input|DisableInput (Variables|Default|GetAs%20Player%20Controller) 0)
  (EventDispatchers|UnbindallEventsfromOnDestroyed))

(event EventBeginPlay
  (bind _healthcomponent (Variables|Default|GetHealthComponent))
  (bind _weapon (Variables|Default|GetWeapon))
  (|CallParentFunction)
  (bind _asplayer_controller (Utilities|Casting|CastToPlayerController (Pawn|GetController))
    (:then
      (Variables|Default|SetAs%20Player%20Controller _asplayer_controller)
      (bind _returnvalue (UserInterface|CreateWidget (Variables|Default|GetHUDClass) _asplayer_controller))
      (bind _output_get (Variables|Default|SetHUDObject _returnvalue))
      (UserInterface|Viewport|AddtoViewport _returnvalue 0)
      (EventDispatchers|BindEventtoOnHurt _healthcomponent (EventDispatchers|CreateEvent _returnvalue :!event SetHealth))
      (EventDispatchers|BindEventtoOnDead _healthcomponent (EventDispatchers|CreateEvent _returnvalue :!event SetHealth))
      ;[1 1 1] Week2
      (EventDispatchers|BindEventtoOnHeal _healthcomponent (EventDispatchers|CreateEvent _returnvalue :!event SetHealth))
      (EventDispatchers|BindEventtoOnAmmoChange _weapon (EventDispatchers|CreateEvent _returnvalue :!event SetAmmo))
      (Default|ReloadAmmo _weapon)
      (EventDispatchers|BindEventtoOnDeathEnded (Variables|Default|GetAs%20ABP%20Character%20Animation) (EventDispatchers|CreateEvent :!event K2DestroyActor)))
    (:CastFailed
      (Development|PrintString "We need a player controller")
      (Actor|DestroyActor))))

(event EventHandleDeath
  (params (Percent :type Float%20%28single-precision%29))
  (|CallParentFunction Percent)
  (Input|DisableInput (Variables|Default|GetAs%20Player%20Controller))
  (Widget|RemovefromParent (Variables|Default|GetHUDObject)))

(event Input|ActionEvents|InputActionAttackInput
  (params (Key :type Key%20Structure :default "None"))
  (:Pressed
    (Default|Attack (Variables|Default|GetWeapon))))

(event Input|ActionEvents|InputActionReloadInput
  (params (Key :type Key%20Structure :default "None"))
  ;[1 1 1] Week2
  (:Pressed
    (Default|RequestReload (Variables|Default|GetWeapon))))

(event Input|AxisEvents|InputAxisTurnRight
  (params (AxisValue :type Float%20%28single-precision%29))
  (Pawn|Input|AddControllerYawInput AxisValue))

(event Input|AxisEvents|InputAxisLookUp
  (params (AxisValue :type Float%20%28single-precision%29))
  (Pawn|Input|AddControllerPitchInput AxisValue))

(event Input|AxisEvents|InputAxisMoveForward
  (params (AxisValue :type Float%20%28single-precision%29))
  (Pawn|Input|AddMovementInput (Math|Vector|GetForwardVector (Math|Rotator|MakeRotator 0.0 0.0 (.Yaw (Math|Rotator|BreakRotator (Pawn|GetControlRotation :!class /Script/Engine.Pawn))))) AxisValue false))

(event Input|AxisEvents|InputAxisStrafe
  (params (AxisValue :type Float%20%28single-precision%29))
  (Pawn|Input|AddMovementInput (Math|Vector|GetRightVector (Math|Rotator|MakeRotator 0.0 0.0 (.Yaw (Math|Rotator|BreakRotator (Pawn|GetControlRotation :!class /Script/Engine.Pawn))))) AxisValue false))

(fn ConstructionScript
  (|CallParentFunction))

(fn CanPickupHealth
  (return true))