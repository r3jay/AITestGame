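; Game mode that tracks the player and enemy characters to decide when the match is won or lost.
; On BeginPlay it sorts all BP_BaseCharacter actors, binds to their OnDestroyed events, counts enemies and creates a results widget.
; When the enemy count reaches zero, it shows the win result and calls WinGame on the player.
; Player destruction shows the results with UI-only input and unbinds enemy destruction events.
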(event Custom|RemoveEnemy
  (params (DestroyedActor :type Actor%20Object%20Reference))
  (bind _resultswidget (Variables|Default|GetResultsWidget))
  (bind _result (Math|Integer|DecrementInt (Variables|Default|GetNumberOfEnemies))
    (:%20%20
      (if (== _result 0)
        (Default|SetWin _resultswidget)
        (UserInterface|Viewport|AddtoViewport _resultswidget 0)
        (Default|WinGame (Variables|Default|GetCurrentPlayer))))))

(event Custom|RemovePlayer
  (params (DestroyedActor :type Actor%20Object%20Reference))
  (bind _currentcontroller (Variables|Default|GetCurrentController))
  (UserInterface|Viewport|AddtoViewport (Variables|Default|GetResultsWidget) 0)
  (Variables|/Script/Engine.PlayerController|SetbShowMouseCursor _currentcontroller true)
  (Input|SetInputModeUIOnly _currentcontroller (Variables|Default|GetResultsWidget) "LockAlways")
  (bind _outactors (Actor|GetAllActorsOfClass "/Game/Blueprints/Actors/BP_BaseCharacter.BP_BaseCharacter_C"))
  (for _array_element _outactors
    (Utilities|Casting|CastToBP_Player _array_element
      (:CastFailed
        (Game|UnbindEventfromOnDestroyed _array_element (EventDispatchers|CreateEvent :!event Custom|RemoveEnemy))))))

(event EventBeginPlay
  (bind _outactors (Actor|GetAllActorsOfClass "/Game/Blueprints/Actors/BP_BaseCharacter.BP_BaseCharacter_C"))
  (for _array_element _outactors
    (bind _asbp_player (Utilities|Casting|CastToBP_Player _array_element)
      (:then
        (Game|BindEventtoOnDestroyed _asbp_player (EventDispatchers|CreateEvent :!event Custom|RemovePlayer))
        (Variables|Default|SetCurrentPlayer _asbp_player))
      (:CastFailed
        (CallFunction|AddEnemy _array_element))))
  (bind _returnvalue (Actor|GetActorOfClass (Variables|Default|GetPlayerControllerClass)))
  (Variables|Default|SetCurrentController _returnvalue)
  (bind _returnvalue_2 (UserInterface|CreateWidget (Variables|Default|GetResultWidgetClass) _returnvalue))
  (Variables|Default|SetResultsWidget _returnvalue_2))

(fn ConstructionScript)

(fn AddEnemy
  (params (Enemy :type Actor%20Object%20Reference))
  (Game|BindEventtoOnDestroyed Enemy (EventDispatchers|CreateEvent :!event Custom|RemoveEnemy))
  (Math|Integer|IncrementInt (Variables|Default|GetNumberOfEnemies)))