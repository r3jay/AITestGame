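; Rifle weapon actor for a parent Pawn that fires projectiles from a muzzle socket along the pawn's aim, destroying itself without a pawn owner.
; Firing requires a living owner, ammo and no ongoing action, then starts a timer and spends a round.
; Reload requests only raise an event and lock actions, with separate events to refill ammo and clear the lock.
; Dispatchers broadcast firing, reload, action-end and ammo changes.
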(event Custom|ActionStopped
  ;[1 1 1] Week 1
  (Variables|Default|SetOnGoing%20Action false)
  (Default|CallOnActionStopped))

(event Custom|OwnerDied
  (Variables|Default|SetOwnerAlive false))

(event Custom|ReloadAmmo
  (bind _max (Variables|Default|GetMax))
  ;[1 1 1] Week 2
  (bind _output_get (Variables|Default|SetCurrent _max))
  (Default|CallOnAmmoChange _output_get _max))

(event Custom|UseAmmo
  ;[1 1 1] Week 2
  (bind _output_get (Variables|Default|SetCurrent (Math|Float|Max(Float) (- (Variables|Default|GetCurrent) 1.0) 0.0)))
  (Default|CallOnAmmoChange _output_get (Variables|Default|GetMax)))

(event Custom|RequestReload
  ;[1 1 1] Week2
  (if (not (Variables|Default|GetOnGoing%20Action))
    (Default|CallOnReloadStart)
    (Variables|Default|SetOnGoing%20Action true)))

(event EventBeginPlay
  (bind _aspawn (Utilities|Casting|CastToPawn (Actor|GetParentActor))
    (:then
      (Variables|Default|SetParentPawn _aspawn)
      (CallFunction|ReloadAmmo) ; Week 2
    )
    (:CastFailed
      (Development|PrintString "Need a pawn to own this gun")
      (Actor|DestroyActor))))

(fn ConstructionScript)

(fn Attack
  (bind _parentpawn (Variables|Default|GetParentPawn))
  (if (CallFunction|CanShoot)
    (Game|SpawnActorfromClass (Variables|Default|GetProjectileClass) (Math|Transform|MakeTransform (Transformation|GetSocketLocation (Variables|Default|GetSkeletalMesh) (Variables|Default|GetSpawn%20Socket%20Name)) (Pawn|GetBaseAimRotation _parentpawn) "1,1,1") "Undefined" (Pawn|GetController _parentpawn) _parentpawn)
    (Variables|Default|SetOnGoing%20Action true)
    (Utilities|Time|SetTimerbyEvent (EventDispatchers|CreateEvent :!event Custom|ActionStopped) 2.0)
    (Default|CallOnWeaponFired)
    (CallFunction|UseAmmo) ; Week 2
  ))

(fn CanShoot
  (return (Math|Boolean|ANDBoolean (not (Variables|Default|GetOnGoing%20Action)) (Variables|Default|GetOwnerAlive) (> (Variables|Default|GetCurrent) 0.0))))