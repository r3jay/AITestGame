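; Game instance Blueprint that handles level switching and quitting for the game.
; Events for the first level, main menu and current level pass stored indices into LoadLevelSafe.
; That function validates the index against the GameLevels array, records it as the current level and opens the level by name, or prints an error if invalid.
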(event Custom|LoadFirstLevel
  (CallFunction|LoadLevelSafe (Variables|Default|GetFirstLevelIndex)))

(event Custom|QuitGame
  (Game|QuitGame 0 "Quit" false))

(event Custom|LoadMainMenu
  (CallFunction|LoadLevelSafe (Variables|Default|GetMainMenuIndex)))

(event Custom|LoadCurrentLevel
  (CallFunction|LoadLevelSafe (Variables|Default|GetCurrentLevelIndex)))

(fn LoadLevelSafe
  (params (LevelIndex :type Integer))
  (if (Utilities|Array|IsValidIndex (Variables|Default|GetGameLevels) LevelIndex)
    (Variables|Default|SetCurrentLevelIndex LevelIndex)
    (Game|OpenLevel(byName) (Utilities|Array|Get(acopy) (Variables|Default|GetGameLevels) LevelIndex))
    (else
      (Development|PrintString (Utilities|String|Append (Utilities|String|ToString(Integer) LevelIndex) "Is not a valid index")))))